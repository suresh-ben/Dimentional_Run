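; Game mode for an endless runner that spawns the track and tracks high score and orb totals.
; BeginPlay loads GameData, shows WBP_Game and chains ten tiles via each NextSpawnPoint, with rare downward drops once StartupTiles runs out.
; Tick updates both totals, then reloads them from the save slot or a fresh save object.
; LoadToGameData copies totals into the save object on player death, without writing to disk.
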(event Custom|LoadGameData
  (bind _returnvalue (SaveGame|DoesSaveGameExist "GameData"))
  (if _returnvalue
    (bind _returnvalue_2 (SaveGame|LoadGamefromSlot "GameData"))
    (bind _asbp_game_data (Utilities|Casting|CastToBP_GameData _returnvalue_2))
    (Variables|Default|SetGameDataInst _asbp_game_data)
    (else
      (bind _returnvalue_3 (SaveGame|CreateSaveGameObject "/Game/_Game/GameManagers/BP_GameData.BP_GameData_C"))
      (Variables|Default|SetGameDataInst _returnvalue_3)))
  (Variables|Default|SetCurrentHighScore (Variables|/Game/_Game/GameManagers/BP_GameData.BP_GameData_C|GetHighScore (Variables|Default|GetGameDataInst)))
  (Variables|Default|SetCurrentTotalOrbs (Variables|/Game/_Game/GameManagers/BP_GameData.BP_GameData_C|GetTotalOrbs (Variables|Default|GetGameDataInst))))

(event Custom|LoadToGameData
  (bind _gamedatainst (Variables|Default|GetGameDataInst))
  (bind _asbp_runner_character (Utilities|Casting|CastToBP_RunnerCharacter (Game|Player|GetPlayerPawn 0)))
  (if (Variables|/Game/_Game/Characters/BP_RunnerCharacter.BP_RunnerCharacter_C|GetisDead _asbp_runner_character)
    (Variables|/Game/_Game/GameManagers/BP_GameData.BP_GameData_C|SetHighScore _gamedatainst (Variables|Default|GetCurrentHighScore))
    (Variables|/Game/_Game/GameManagers/BP_GameData.BP_GameData_C|SetTotalOrbs _gamedatainst (Variables|Default|GetCurrentTotalOrbs))))

(event EventBeginPlay
  (CallFunction|LoadGameData)
  (bind _returnvalue (UserInterface|CreateWidget "/Game/_Game/Assets/Ui/WBP_Game.WBP_Game_C"))
  (bind _output_get (Variables|Default|SetGameUi _returnvalue))
  (bind _output_get_2 (Variables|Default|SetGame%20Widget _output_get))
  (UserInterface|Viewport|AddtoViewport _output_get_2 0)
  (for _index (range 0 9)
    (CallFunction|SpawnTile)))

(event EventTick
  (params (DeltaSeconds :type Float%20%28single-precision%29))
  (CallFunction|SetHighScoreandCoins)
  (CallFunction|LoadGameData))

(fn ConstructionScript)

(fn SpawnTile
  (if (and (<= (Variables|Default|GetStartupTiles) 0) (> (Math|Random|RandomFloat) 0.95))
    (Variables|Default|SetNextTileSpawnPoint (Math|Transform|MakeTransform (Math|Vector|MakeVector (.x (.location (Variables|Default|GetNextTileSpawnPoint))) (.y (.location (Variables|Default|GetNextTileSpawnPoint))) (- (.z (.location (Variables|Default|GetNextTileSpawnPoint))) 5e+02)) (.rotation (Variables|Default|GetNextTileSpawnPoint)) (.scale (Variables|Default|GetNextTileSpawnPoint)))))
  (bind _returnvalue (Game|SpawnActorfromClass "/Game/_Game/Assets/Spawns/Tiles/BP_MasterTile.BP_MasterTile_C" (Variables|Default|GetNextTileSpawnPoint) "Undefined" 0 0))
  (Variables|Default|SetNextTileSpawnPoint (Math|Transform|MakeTransform (Transformation|GetWorldLocation (Variables|/Game/_Game/Assets/Spawns/Tiles/BP_MasterTile.BP_MasterTile_C|GetNextSpawnPoint _returnvalue)) "0, 0, 0" "1,1,1")))

(fn SetHighScoreandCoins
  (if (> (Variables|Default|GetcurrentPoints) (Variables|Default|GetCurrentHighScore))
    (Variables|Default|SetCurrentHighScore (Variables|Default|GetcurrentPoints)))
  (Variables|Default|SetCurrentTotalOrbs (+ (Variables|Default|GetcurrentCoins) (Variables|Default|GetCurrentTotalOrbs))))
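; BP_MasterTile is a track tile for a runner game that keeps the track extending as the player advances.
; On BeginPlay it spawns an Orb actor at the Lane0 transform.
; When BP_RunnerCharacter overlaps SpawnerCollision, it asks BP_DimentionalRun_GameMode to spawn another tile, then destroys itself after a short delay.
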(event OnComponentBeginOverlap(SpawnerCollision)
  (params (OverlappedComponent :type Primitive%20Component%20Object%20Reference) (OtherActor :type Actor%20Object%20Reference) (OtherComp :type Primitive%20Component%20Object%20Reference) (OtherBodyIndex :type Integer) (bFromSweep :type Boolean) (SweepResult :type Hit%20Result%20Structure%20%28by%20ref%29))
  (Utilities|Casting|CastToBP_RunnerCharacter OtherActor)
  (bind _asbp_dimentional_run_game_mode (Utilities|Casting|CastToBP_DimentionalRun_GameMode (Game|GetGameMode)))
  (Default|SpawnTile _asbp_dimentional_run_game_mode)
  (Utilities|FlowControl|Delay 1.0)
  (Actor|DestroyActor))

(event EventBeginPlay
  (CallFunction|SpawnActors))

(event Collision|EventActorBeginOverlap
  (params (OtherActor :type Actor%20Object%20Reference)))

(event EventTick
  (params (DeltaSeconds :type Float%20%28single-precision%29)))

(fn ConstructionScript)

(fn SpawnActors
  (Game|SpawnActorfromClass "/Game/_Game/Assets/Orbs/Materials/Orb.Orb_C" (Transformation|GetWorldTransform (Variables|Default|GetLane%200)) "Undefined" 0 0))
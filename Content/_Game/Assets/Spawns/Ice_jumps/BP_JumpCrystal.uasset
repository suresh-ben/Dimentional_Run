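; BP_JumpCrystal is a spawner that places a randomly chosen ice crystal obstacle for the runner character.
; On BeginPlay it picks one of seven crystal variants, spawns it at the spawn point component's transform and stores it as Block.
; When a runner overlaps CollisionManager, Block's collision is disabled if the runner has super run and enabled otherwise, letting super runs pass through.
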(event OnComponentBeginOverlap(CollisionManager)
  (params (OverlappedComponent :type Primitive%20Component%20Object%20Reference) (OtherActor :type Actor%20Object%20Reference) (OtherComp :type Primitive%20Component%20Object%20Reference) (OtherBodyIndex :type Integer) (bFromSweep :type Boolean) (SweepResult :type Hit%20Result%20Structure%20%28by%20ref%29))
  (bind _asbp_runner_character (Utilities|Casting|CastToBP_RunnerCharacter OtherActor))
  (if (Variables|/Game/_Game/Characters/BP_RunnerCharacter.BP_RunnerCharacter_C|GethasSuperRun _asbp_runner_character)
    (Collision|SetActorEnableCollision (Variables|Default|GetBlock) false)
    (else
      (Collision|SetActorEnableCollision (Variables|Default|GetBlock) true))))

(event EventBeginPlay
  (bind _sapwnpoint (Variables|Default|GetSapwnPoint))
  (bind _returnvalue (Transformation|GetWorldTransform _sapwnpoint))
  (switch int (Math|Random|RandomIntegerinRange 0 6)
    (:0
      (bind _returnvalue_2 (Game|SpawnActorfromClass "/Game/_Game/Assets/Spawns/Ice_jumps/Models/BP_s/BP_crystal_01.BP_crystal_01_C" _returnvalue "Undefined" 0 0))
      (Variables|Default|SetBlock _returnvalue_2))
    (:1
      (bind _returnvalue_3 (Game|SpawnActorfromClass "/Game/_Game/Assets/Spawns/Ice_jumps/Models/BP_s/BP_crystal_02.BP_crystal_02_C" _returnvalue "Undefined" 0 0))
      (Variables|Default|SetBlock _returnvalue_3))
    (:2
      (bind _returnvalue_4 (Game|SpawnActorfromClass "/Game/_Game/Assets/Spawns/Ice_jumps/Models/BP_s/BP_crystal_03.BP_crystal_03_C" _returnvalue "Undefined" 0 0))
      (Variables|Default|SetBlock _returnvalue_4))
    (:3
      (bind _returnvalue_5 (Game|SpawnActorfromClass "/Game/_Game/Assets/Spawns/Ice_jumps/Models/BP_s/BP_crystal_04.BP_crystal_04_C" _returnvalue "Undefined" 0 0))
      (Variables|Default|SetBlock _returnvalue_5))
    (:4
      (bind _returnvalue_6 (Game|SpawnActorfromClass "/Game/_Game/Assets/Spawns/Ice_jumps/Models/BP_s/BP_crystal_05.BP_crystal_05_C" _returnvalue "Undefined" 0 0))
      (Variables|Default|SetBlock _returnvalue_6))
    (:5
      (bind _returnvalue_7 (Game|SpawnActorfromClass "/Game/_Game/Assets/Spawns/Ice_jumps/Models/BP_s/BP_crystal_06.BP_crystal_06_C" _returnvalue "Undefined" 0 0))
      (Variables|Default|SetBlock _returnvalue_7))
    (:6
      (bind _returnvalue_8 (Game|SpawnActorfromClass "/Game/_Game/Assets/Spawns/Ice_jumps/Models/BP_s/BP_crystal_07.BP_crystal_07_C" _returnvalue "Undefined" 0 0))
      (Variables|Default|SetBlock _returnvalue_8))))

(event Collision|EventActorBeginOverlap
  (params (OtherActor :type Actor%20Object%20Reference)))

(event EventTick
  (params (DeltaSeconds :type Float%20%28single-precision%29)))

(fn ConstructionScript)
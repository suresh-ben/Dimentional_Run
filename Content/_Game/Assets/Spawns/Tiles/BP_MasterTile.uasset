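; Track tile for the runner game that places a random item and keeps the track extending as the player advances.
; On BeginPlay, SpawnActors spawns one of Orb, jump crystal, ice block or pillar at Lane0, with equal odds.
; When BP_RunnerCharacter overlaps SpawnerCollision, the tile asks the game mode to spawn another tile, then destroys itself after a short delay.
; Spawned items are not attached or tracked, so the tile does not remove them.
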(event OnComponentBeginOverlap(SpawnerCollision)
  (params (OverlappedComponent :type Primitive%20Component%20Object%20Reference) (OtherActor :type Actor%20Object%20Reference) (OtherComp :type Primitive%20Component%20Object%20Reference) (OtherBodyIndex :type Integer) (bFromSweep :type Boolean) (SweepResult :type Hit%20Result%20Structure%20%28by%20ref%29))
  (Utilities|Casting|CastToBP_RunnerCharacter OtherActor)
  (bind _asbp_dimentional_run_game_mode (Utilities|Casting|CastToBP_DimentionalRun_GameMode (Game|GetGameMode)))
  (Default|SpawnTile _asbp_dimentional_run_game_mode)
  (Utilities|FlowControl|Delay 1.0)
  (Actor|DestroyActor))

(event EventBeginPlay
  (CallFunction|SpawnActors))

(event Collision|EventActorBeginOverlap
  (params (OtherActor :type Actor%20Object%20Reference)))

(event EventTick
  (params (DeltaSeconds :type Float%20%28single-precision%29)))

(fn ConstructionScript)

(fn SpawnActors
  (bind _lane_0 (Variables|Default|GetLane%200))
  (bind _returnvalue (Transformation|GetWorldTransform _lane_0))
  (switch int (Math|Random|RandomIntegerinRange 0 3)
    (:0
      (Game|SpawnActorfromClass "/Game/_Game/Assets/Spawns/Orbs/Orb.Orb_C" _returnvalue "Undefined" 0 0))
    (:1
      (Game|SpawnActorfromClass "/Game/_Game/Assets/Spawns/Ice_jumps/BP_JumpCrystal.BP_JumpCrystal_C" _returnvalue "Undefined" 0 0))
    (:2
      (Game|SpawnActorfromClass "/Game/_Game/Assets/Spawns/ice_Blocks/BP_Ice_Block.BP_Ice_Block_C" _returnvalue "Undefined" 0 0))
    (:3
      (Game|SpawnActorfromClass "/Game/_Game/Assets/Spawns/Pillar/BP_Pillar.BP_Pillar_C" _returnvalue "Undefined" 0 0))))
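; BP_Orb is a coin pickup that adds one to the game mode's CurrentCoins and destroys itself when the runner's character overlaps its mesh.
; A separate MagnetManager overlap flags the orb to home in on the player if that runner has magnets.
; While flagged, Tick lerps the orb's root toward the player each frame, with alpha scaled by DeltaSeconds and the player's MaxWalkSpeed.
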(event OnComponentBeginOverlap(StaticMesh)
  (params (OverlappedComponent :type Primitive%20Component%20Object%20Reference) (OtherActor :type Actor%20Object%20Reference) (OtherComp :type Primitive%20Component%20Object%20Reference) (OtherBodyIndex :type Integer) (bFromSweep :type Boolean) (SweepResult :type Hit%20Result%20Structure%20%28by%20ref%29))
  (Utilities|Casting|CastToBP_RunnerCharacter OtherActor)
  (bind _asbp_dimentional_run_game_mode (Utilities|Casting|CastToBP_DimentionalRun_GameMode (Game|GetGameMode)))
  (Variables|/Game/_Game/GameManagers/BP_DimentionalRun_GameMode.BP_DimentionalRun_GameMode_C|SetcurrentCoins _asbp_dimentional_run_game_mode (+ (Variables|/Game/_Game/GameManagers/BP_DimentionalRun_GameMode.BP_DimentionalRun_GameMode_C|GetcurrentCoins _asbp_dimentional_run_game_mode) 1))
  (Actor|DestroyActor))

(event OnComponentBeginOverlap(MagnetManager)
  (params (OverlappedComponent :type Primitive%20Component%20Object%20Reference) (OtherActor :type Actor%20Object%20Reference) (OtherComp :type Primitive%20Component%20Object%20Reference) (OtherBodyIndex :type Integer) (bFromSweep :type Boolean) (SweepResult :type Hit%20Result%20Structure%20%28by%20ref%29))
  (bind _asbp_runner_character (Utilities|Casting|CastToBP_RunnerCharacter OtherActor))
  (if (Variables|/Game/_Game/Characters/BP_RunnerCharacter.BP_RunnerCharacter_C|GethasMagnets _asbp_runner_character)
    (Variables|Default|SetcanMovetoPlayer true)))

(event EventTick
  (params (DeltaSeconds :type Float%20%28single-precision%29))
  (if (Variables|Default|GetcanMovetoPlayer)
    (bind _asbp_runner_character (Utilities|Casting|CastToBP_RunnerCharacter (Game|Player|GetPlayerPawn 0)))
    (Transformation|SetWorldLocation (Variables|Default|GetDefaultSceneRoot) (Math|Vector|MakeVector (.x (Math|Vector|Lerp(Vector) (Transformation|GetWorldLocation (Variables|Default|GetDefaultSceneRoot)) (Transformation|GetWorldLocation (Variables|/Script/Engine.Actor|GetRootComponent _asbp_runner_character)) (* DeltaSeconds (/ (Variables|/Script/Engine.CharacterMovementComponent|GetMaxWalkSpeed (Variables|/Script/Engine.Character|GetCharacterMovement _asbp_runner_character)) 1e+02)))) (.y (Math|Vector|Lerp(Vector) (Transformation|GetWorldLocation (Variables|Default|GetDefaultSceneRoot)) (Transformation|GetWorldLocation (Variables|/Script/Engine.Actor|GetRootComponent _asbp_runner_character)) (* DeltaSeconds (/ (Variables|/Script/Engine.CharacterMovementComponent|GetMaxWalkSpeed (Variables|/Script/Engine.Character|GetCharacterMovement _asbp_runner_character)) 1e+02)))) (.z (Math|Vector|Lerp(Vector) (Transformation|GetWorldLocation (Variables|Default|GetDefaultSceneRoot)) (Transformation|GetWorldLocation (Variables|/Script/Engine.Actor|GetRootComponent _asbp_runner_character)) (* DeltaSeconds (/ (Variables|/Script/Engine.CharacterMovementComponent|GetMaxWalkSpeed (Variables|/Script/Engine.Character|GetCharacterMovement _asbp_runner_character)) 1e+02))))) false false)))

(fn ConstructionScript)
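; BP_Ice_Block is a spawner that places one randomly chosen block variant when play begins.
; BeginPlay rolls a random integer and spawns one of six classes, BP_Block_01 to BP_Block_06, at the SpawnPoint component's world transform.
; It then assigns SpawnPoint to the spawned block's DefaultSceneRoot variable, with no explicit attach call.
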(event EventBeginPlay
  (bind _spawnpoint (Variables|Default|GetSpawnPoint))
  (bind _returnvalue (Transformation|GetWorldTransform _spawnpoint))
  (switch int (Math|Random|RandomIntegerinRange 0 5)
    (:0
      (bind _returnvalue_2 (Game|SpawnActorfromClass "/Game/_Game/Assets/Spawns/ice_Blocks/Models/BP_s/BP_Block_01.BP_Block_01_C" _returnvalue "Undefined" 0 0))
      (Variables|/Game/_Game/Assets/Spawns/ice_Blocks/Models/BP_s/BP_Block_01.BP_Block_01_C|SetDefaultSceneRoot _returnvalue_2 (Variables|Default|GetSpawnPoint)))
    (:1
      (bind _returnvalue_3 (Game|SpawnActorfromClass "/Game/_Game/Assets/Spawns/ice_Blocks/Models/BP_s/BP_Block_02.BP_Block_02_C" _returnvalue "Undefined" 0 0))
      (Variables|/Game/_Game/Assets/Spawns/ice_Blocks/Models/BP_s/BP_Block_02.BP_Block_02_C|SetDefaultSceneRoot _returnvalue_3 (Variables|Default|GetSpawnPoint)))
    (:2
      (bind _returnvalue_4 (Game|SpawnActorfromClass "/Game/_Game/Assets/Spawns/ice_Blocks/Models/BP_s/BP_Block_03.BP_Block_03_C" _returnvalue "Undefined" 0 0))
      (Variables|/Game/_Game/Assets/Spawns/ice_Blocks/Models/BP_s/BP_Block_03.BP_Block_03_C|SetDefaultSceneRoot _returnvalue_4 (Variables|Default|GetSpawnPoint)))
    (:3
      (bind _returnvalue_5 (Game|SpawnActorfromClass "/Game/_Game/Assets/Spawns/ice_Blocks/Models/BP_s/BP_Block_04.BP_Block_04_C" _returnvalue "Undefined" 0 0))
      (Variables|/Game/_Game/Assets/Spawns/ice_Blocks/Models/BP_s/BP_Block_04.BP_Block_04_C|SetDefaultSceneRoot _returnvalue_5 (Variables|Default|GetSpawnPoint)))
    (:4
      (bind _returnvalue_6 (Game|SpawnActorfromClass "/Game/_Game/Assets/Spawns/ice_Blocks/Models/BP_s/BP_Block_05.BP_Block_05_C" _returnvalue "Undefined" 0 0))
      (Variables|/Game/_Game/Assets/Spawns/ice_Blocks/Models/BP_s/BP_Block_05.BP_Block_05_C|SetDefaultSceneRoot _returnvalue_6 (Variables|Default|GetSpawnPoint)))
    (:5
      (bind _returnvalue_7 (Game|SpawnActorfromClass "/Game/_Game/Assets/Spawns/ice_Blocks/Models/BP_s/BP_Block_06.BP_Block_06_C" _returnvalue "Undefined" 0 0))
      (Variables|/Game/_Game/Assets/Spawns/ice_Blocks/Models/BP_s/BP_Block_06.BP_Block_06_C|SetDefaultSceneRoot _returnvalue_7 (Variables|Default|GetSpawnPoint)))))

(event Collision|EventActorBeginOverlap
  (params (OtherActor :type Actor%20Object%20Reference)))

(event EventTick
  (params (DeltaSeconds :type Float%20%28single-precision%29)))

(fn ConstructionScript)